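; Base weapon for a third-person shooter, handling start/stop fire, aiming and cosmetic fire effects.
; StartFire is gated by WantsToFire, playing fire audio, tracing aim, then spawning hit sound and emitter once per press.
; CameraAim traces Visibility from the muzzle socket toward a distant point on the camera aim line.
; AimVector receives the hit location, or a muzzle-relative offset on a miss; no damage is applied.
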(fn `CameraAim`
  (bind _muzzlelocation (`self.GetMuzzleLocation`))
  (bind _ownercomponent (`self.OwnerComponent`))
  (bind _tpsplayer_controller (`/Game/Main/Components/WeaponComponent.GetCastedOwner` _ownercomponent))
  (bind _returnvalue (+ (`/Game/Main/TPSPlayerController.GetViewpoint` _tpsplayer_controller) (* (`/Game/Main/TPSPlayerController.GetAimVector` _tpsplayer_controller) 100000.0)))
  (set `self.AimVector` (`KismetMathLibrary.GetForwardVector` (`Pawn.GetBaseAimRotation` (`/Game/Main/Components/WeaponComponent.OwnedActor` _ownercomponent))))
  (bind _outhit (`KismetSystemLibrary.LineTraceSingle` _muzzlelocation _returnvalue "TraceTypeQuery1"))
  (bind (_bblockinghit _binitialoverlap _time _location) (`GameplayStatics.BreakHitResult` _outhit))
  (set `self.AimVector` (`KismetMathLibrary.SelectVector` _location (- _returnvalue _muzzlelocation) _bblockinghit))
  (return))

(fn `FireHitEffect`
  (bind _firehitemitter (`self.FireHitEmitter`))
  (bind _aimvector (`self.AimVector`))
  (bind _firehitsound (`self.FireHitSound`))
  (`|ExecutionSequence`
    (:`then_0`
      (`/Engine/EditorBlueprintResources/StandardMacros.IsValid` _firehitsound
        (:`Is Valid`
          (`GameplayStatics.PlaySoundAtLocation` _firehitsound _aimvector))))
    (:`then_1`
      (`/Engine/EditorBlueprintResources/StandardMacros.IsValid` _firehitemitter
        (:`Is Valid`
          (`GameplayStatics.SpawnEmitterAtLocation` _firehitemitter _aimvector))))))

(fn `FireWeaponEffect`
  (bind _firesound (`self.FireSound`))
  (`/Engine/EditorBlueprintResources/StandardMacros.IsValid` _firesound
    (:`Is Valid`
      (`AudioComponent.Play` _firesound 0.0))))

(fn `GetMuzzleLocation`
  (returns (MuzzleLocation :type "Vector Structure"))
  (return (`SceneComponent.GetSocketLocation` (`self.WeaponMesh`) (`self.MuzzleSocket`))))

(fn `StartFire`
  (if (not (`self.WantsToFire`))
    (set `self.WantsToFire` true)
    (`self.FireWeaponEffect`)
    (`self.CameraAim`)
    (`self.FireHitEffect`)))

(fn `StopFire`
  (if (`self.WantsToFire`)
    (set `self.WantsToFire` false)))

(fn `UserConstructionScript`)